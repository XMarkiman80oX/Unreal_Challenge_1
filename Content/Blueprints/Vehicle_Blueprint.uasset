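; Player vehicle Blueprint that carries materials between factories.
; On BeginPlay it creates the HUD widget and adds it to the viewport.
; Overlapping a GenericFactory with its Box shows a loading/unloading indicator and passes the factory's materials to SuppliesManager.
; If that factory is also a PreReqFactory, SuppliesManager then delivers its required materials, and ending any overlap hides the indicator.
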(event `self.ReceiveBeginPlay`
  (bind _returnvalue (`|CreateWidget` "/Game/UI/HUD.HUD_C"))
  (bind _output_get (set `self.HUD` _returnvalue))
  (`UserWidget.AddToViewport` _output_get 0))

(event `self.Box.OnComponentBeginOverlap`
  (params (OverlappedComponent :type "PrimitiveComponent Object Reference") (OtherActor :type "Actor Object Reference") (OtherComp :type "PrimitiveComponent Object Reference") (OtherBodyIndex :type Integer) (bFromSweep :type Boolean) (SweepResult :type "HitResult Structure (by ref)"))
  (bind _asgeneric_factory (cast `GenericFactory` OtherActor))
  (`SceneComponent.SetVisibility` (`self.Loading/Unloading Status`) true false)
  (`GenericFactory.GetFactoryType` _asgeneric_factory)
  (bind _returnvalue (`GenericFactory.SendMaterials` _asgeneric_factory))
  (`SuppliesManager.CollectMaterials` (`self.SuppliesManager`) _returnvalue)
  (bind _aspre_req_factory (cast `PreReqFactory` OtherActor))
  (bind _returnvalue_2 (`PreReqFactory.GetRequiredMaterials` _aspre_req_factory))
  (bind _returnvalue_3 (`SuppliesManager.SendRequiredMaterials` (`self.SuppliesManager`) _returnvalue_2))
  (`PreReqFactory.ReceiveMaterials` _aspre_req_factory _returnvalue_3))

(event `self.Box.OnComponentEndOverlap`
  (params (OverlappedComponent :type "PrimitiveComponent Object Reference") (OtherActor :type "Actor Object Reference") (OtherComp :type "PrimitiveComponent Object Reference") (OtherBodyIndex :type Integer))
  (`SceneComponent.SetVisibility` (`self.Loading/Unloading Status`) false false))

(fn `UserConstructionScript`)